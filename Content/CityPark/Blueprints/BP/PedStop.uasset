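; Pedestrian stop volume that halts or hurries Pedestrian actors, apparently for traffic control.
; When a pedestrian begins overlapping Box, a check against the second volume, Box1, makes those already inside it run and all others stop.
; The TrafficStop flag on each pedestrian is set on stopping and cleared on running.
; Leaving Box returns the pedestrian to walking and clears the flag.
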(event OnComponentEndOverlap(Box)
  (params (OverlappedComponent :type Primitive%20Component%20Object%20Reference) (OtherActor :type Actor%20Object%20Reference) (OtherComp :type Primitive%20Component%20Object%20Reference) (OtherBodyIndex :type Integer))
  (bind _aspedestrian (Utilities|Casting|CastToPedestrian OtherActor))
  (Default|Walk _aspedestrian)
  (Variables|/Game/CityPark/Blueprints/BP/Pedestrian.Pedestrian_C|SetTraffic%20Stop _aspedestrian false))

(event OnComponentBeginOverlap(Box)
  (params (OverlappedComponent :type Primitive%20Component%20Object%20Reference) (OtherActor :type Actor%20Object%20Reference) (OtherComp :type Primitive%20Component%20Object%20Reference) (OtherBodyIndex :type Integer) (bFromSweep :type Boolean) (SweepResult :type Hit%20Result%20Structure%20%28by%20ref%29))
  (bind _aspedestrian (Utilities|Casting|CastToPedestrian OtherActor))
  (if (Collision|IsOverlappingActor (Variables|Default|GetBox1) _aspedestrian :!class /Script/Engine.PrimitiveComponent)
    (Default|Run _aspedestrian)
    (Variables|/Game/CityPark/Blueprints/BP/Pedestrian.Pedestrian_C|SetTraffic%20Stop _aspedestrian false)
    (else
      (Default|Stop _aspedestrian)
      (Variables|/Game/CityPark/Blueprints/BP/Pedestrian.Pedestrian_C|SetTraffic%20Stop _aspedestrian true))))

(fn ConstructionScript)