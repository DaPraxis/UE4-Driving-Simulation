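; AI traffic car for the city park that steers along an assigned spline, using a look-ahead point on the path.
; A one-second timer runs a stop/drive/decelerate state machine that nudges throttle toward the speed limit or eases off.
; Every tick, overlap boxes trigger a handbrake stop for pedestrians, players or cars, or deceleration, and resume after clearing.
; Text renders show speed, throttle and state for debugging.
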(event Custom|SetSpeed
  (bind _vehiclemovement (Variables|Default|GetVehicleMovement))
  (bind _speed_limit_from_splin (Variables|Default|GetSpeed%20Limit%20From%20Splin))
  (bind _speedthres (Variables|Default|GetSpeedThres))
  (bind _returnvalue (Class|WheeledVehicleMovementComponent|GetForwardSpeed _vehiclemovement))
  (bind _returnvalue_2 (* _returnvalue 0.036))
  (bind _returnvalue_3 (- _speed_limit_from_splin _returnvalue_2))
  (if (not (Variables|Default|GetStand))
    (if (not (Math|Float|InRange(Float) _returnvalue_2 (- _speed_limit_from_splin _speedthres) (+ _speed_limit_from_splin _speedthres)))
      (if (> _returnvalue_3 0.0)
        (Variables|Default|SetThrottle (+ (/ _returnvalue_3 5e+02) (Variables|Default|GetThrottle)))
        (else
          (Variables|Default|SetThrottle (+ (/ _returnvalue_3 8e+01) (Variables|Default|GetThrottle)))))
      (Class|WheeledVehicleMovementComponent|SetThrottleInput (Variables|Default|GetVehicleMovement) (Variables|Default|GetThrottle)))))

(event Custom|Check%20NPC
  (bind _pedbox (Variables|Default|GetPedBox))
  (if (or (> (Utilities|Array|Length (Collision|GetOverlappingActors _pedbox "/Game/CityPark/Blueprints/BP/Pedestrian.Pedestrian_C" :!class /Script/Engine.PrimitiveComponent)) 0) (> (Utilities|Array|Length (Collision|GetOverlappingActors _pedbox "/Game/ThirdPersonBP/Blueprints/ThirdPersonCharacter.ThirdPersonCharacter_C" :!class /Script/Engine.PrimitiveComponent)) 0))
    (CallFunction|Stop)
    (Variables|Default|Setped%20stand true)
    (else
      (Variables|Default|Setped%20stand false)
      (if (not (Math|Boolean|ORBoolean (Variables|Default|Getped%20stand) (Variables|Default|Getveh%20stand) (Variables|Default|Gettraffic_stand)))
        (switch int (Variables|Default|Getdriving%20state) ; If current is stop (1), we can reset
          (:Default
            (Utilities|FlowControl|Delay 1.0 :!label _label)
            (CallFunction|ResetDriving))
          (:1
            (goto _label))
          (:2
            (CallFunction|CheckDec)))))))

(event Custom|Check%20Veh
  (if (> (Utilities|Array|Length (Collision|GetOverlappingActors (Variables|Default|GetVehBox) "AI_Car_C" :!class /Script/Engine.PrimitiveComponent)) 0)
    (CallFunction|Stop)
    (Variables|Default|Setveh%20stand true)
    (else
      (Variables|Default|Setveh%20stand false)
      (if (not (Math|Boolean|ORBoolean (Variables|Default|Getped%20stand) (Variables|Default|Getveh%20stand) (Variables|Default|Gettraffic_stand))) ; Free to resume
        (switch int (Variables|Default|Getdriving%20state) ; If current is stop (1), we can reset
          (:Default
            (Utilities|FlowControl|Delay 1.0 :!label _label)
            (CallFunction|ResetDriving))
          (:1
            (goto _label))
          (:2
            (CallFunction|CheckDec)))))))

(event Custom|Check%20Dec
  (bind _decbox (Variables|Default|GetDecBox))
  (if (Math|Boolean|ORBoolean (> (Utilities|Array|Length (Collision|GetOverlappingActors _decbox "/Game/CityPark/Blueprints/BP/Pedestrian.Pedestrian_C" :!class /Script/Engine.PrimitiveComponent)) 0) (> (Utilities|Array|Length (Collision|GetOverlappingActors _decbox "/Game/ThirdPersonBP/Blueprints/ThirdPersonCharacter.ThirdPersonCharacter_C" :!class /Script/Engine.PrimitiveComponent)) 0) (> (Utilities|Array|Length (Collision|GetOverlappingActors _decbox "AI_Car_C" :!class /Script/Engine.PrimitiveComponent)) 0) (> (Utilities|Array|Length (Collision|GetOverlappingActors _decbox "/Game/CityPark/Blueprints/BP/CarStop.CarStop_C" :!class /Script/Engine.PrimitiveComponent)) 0))
    (Variables|Default|Setdriving%20state 3)))

(event Custom|GameLoop
  (bind _textrender3 (Variables|Default|GetTextRender3))
  (switch int (Variables|Default|Getdriving%20state)
    (:1
      (Rendering|Components|TextRender|SetText _textrender3 (Utilities|Text|ToText(String) "Stop!")))
    (:2
      (CallFunction|SetSpeed)
      (Rendering|Components|TextRender|SetText _textrender3 (Utilities|Text|ToText(String) "Driving!")))
    (:3
      (CallFunction|Dec)
      (Rendering|Components|TextRender|SetText _textrender3 (Utilities|Text|ToText(String) "Dec!")))))

(event EventBeginPlay
  (bind _returnvalue (Components|GetOwner))
  (bind _mesh (Variables|Character|GetMesh))
  ;[1 1 1] Throttle input
  (CallFunction|Spawn)
  (CallFunction|ResetDriving)
  (Class|PrimitiveComponent|IgnoreComponentwhenMoving (Variables|Default|GetDecBox) _mesh true)
  (Collision|IgnoreActorwhenMoving (Variables|Default|GetDecBox) _returnvalue true)
  (Class|PrimitiveComponent|IgnoreComponentwhenMoving (Variables|Default|GetPedBox) _mesh true)
  (Collision|IgnoreActorwhenMoving (Variables|Default|GetPedBox) _returnvalue true)
  (Class|PrimitiveComponent|IgnoreComponentwhenMoving (Variables|Default|GetVehBox) _mesh true)
  (Collision|IgnoreActorwhenMoving (Variables|Default|GetVehBox) _returnvalue true)
  (Utilities|Time|SetTimerbyEvent (delegate Custom|GameLoop) 1.0 true))

(event EventTick
  (params (DeltaSeconds :type Float%20%28single-precision%29))
  (bind _steeringthre (Variables|Default|GetSteeringThre))
  ;[1 1 1] Steering input
  (bind _steering (CallFunction|GetPath))
  (if (Math|Float|InRange(Float) _steering (- (Variables|Default|GetSteering) _steeringthre) (+ (Variables|Default|GetSteering) _steeringthre))
    _
    (else
      (Class|WheeledVehicleMovementComponent|SetSteeringInput (Variables|Default|GetVehicleMovement) _steering)
      (Variables|Default|SetSteering _steering)))
  (CallFunction|CheckNPC)
  (CallFunction|CheckVeh)
  (Rendering|Components|TextRender|SetText (Variables|Default|GetTextRender) (Utilities|Text|ToText(Float) (* (Class|WheeledVehicleMovementComponent|GetForwardSpeed (Variables|Default|GetVehicleMovement)) 0.036) "HalfToEven"))
  (Rendering|Components|TextRender|SetText (Variables|Default|GetTextRender1) (Utilities|Text|ToText(Float) (Variables|Default|GetThrottle) "HalfToEven"))
  (Rendering|Components|TextRender|SetText (Variables|Default|GetTextRender2) (Utilities|Text|ToText(Boolean) (Variables|Default|Gettraffic_stand))))

(fn ConstructionScript)

(fn GetPath
  (bind _returnvalue (Transformation|GetActorLocation))
  (bind _active_path (Variables|Default|GetActive%20Path))
  (Utilities|IsValid _active_path
    (:Is%20Valid
      (return (Math|Float|MapRangeClamped (.yaw (Math|Rotator|Delta(Rotator) (Math|Rotator|FindLookatRotation _returnvalue (Spline|FindLocationClosesttoWorldLocation _active_path (+ (* (Math|Vector|Normalize (Class|SplineComponent|FindTangentClosesttoWorldLocation _active_path _returnvalue "World")) 5e+02) _returnvalue) "World")) (Transformation|GetActorRotation))) -9e+01 9e+01 -1.0 1.0)))))

(fn Stop
  (bind _vehiclemovement (Variables|Default|GetVehicleMovement))
  (Class|WheeledVehicleMovementComponent|SetThrottleInput _vehiclemovement -1.0)
  (bind _output_get (Variables|Default|SetStand true))
  (Class|WheeledVehicleMovementComponent|SetHandbrakeInput _vehiclemovement _output_get)
  (Variables|Default|SetThrottle (Variables|Default|GetReset%20Throttle))
  (Variables|Default|Setdriving%20state 1))

(fn ResetDriving
  (bind _vehiclemovement (Variables|Default|GetVehicleMovement))
  (bind _output_get (Variables|Default|SetStand false))
  (Class|WheeledVehicleMovementComponent|SetHandbrakeInput _vehiclemovement _output_get)
  (bind _output_get_2 (Variables|Default|SetThrottle (Variables|Default|GetThrottle)))
  (Class|WheeledVehicleMovementComponent|SetThrottleInput _vehiclemovement _output_get_2)
  (Class|WheeledVehicleMovementComponent|SetBrakeInput _vehiclemovement 0.0)
  (Variables|Default|Setdriving%20state 2))

(fn Spawn
  (bind _mesh (Variables|Character|GetMesh))
  (Class|SkinnedMeshComponent|SetSkeletalMesh _mesh (Variables|Default|GetSkMesh) false)
  (Class|SkeletalMeshComponent|SetAnimClass _mesh (Variables|Default|GetAnim))
  (Class|WheeledVehicleMovementComponent|SetSteeringInput (Variables|Default|GetVehicleMovement) (Variables|Default|GetSteering)))

(fn Dec
  (bind _vehiclemovement (Variables|Default|GetVehicleMovement))
  (bind _returnvalue (Class|WheeledVehicleMovementComponent|GetForwardSpeed _vehiclemovement))
  (if (> _returnvalue 0.0)
    (if (Math|Float|InRange(Float) (* _returnvalue 0.036) 0.0 (Variables|Default|GetDec%20Target%20Speed))
      (Variables|Default|Setdriving%20state 2 :!label _label)
      (else
        (Class|WheeledVehicleMovementComponent|SetThrottleInput (Variables|Default|GetVehicleMovement) 0.2)))
    (else
      (goto _label))))