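; Pedestrian character for CityPark that takes a random human mesh at BeginPlay, starts at walking speed and halts for nearby cars.
; Every Tick it checks VehBox for overlapping AI_Car actors, stopping while any are present and resuming otherwise unless TrafficStop is set.
; Stop, Walk, Run and Resume drive MaxWalkSpeed, with CurrentSpeed remembering the gait to restore.
; The random index range leaves the sixth mesh (Sophia) unused.
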(event Custom|CheckVeh
  (if (> (Utilities|Array|Length (Collision|GetOverlappingActors (Variables|Default|GetVehBox) "/Game/CityPark/Blueprints/BP/AI_Car.AI_Car_C" :!class /Script/Engine.PrimitiveComponent)) 0)
    (CallFunction|Stop)
    (Variables|Default|Setveh%20stand true)
    (else
      (Variables|Default|Setveh%20stand false)
      (if (not (Variables|Default|GetTraffic%20Stop))
        (CallFunction|Resume)))))

(event EventBeginPlay
  (Class|SkinnedMeshComponent|SetSkeletalMesh (Variables|Character|GetMesh) (Utilities|Select :Index (Math|Random|RandomInteger 5) :Option%200 "/Game/CityPark/Blueprints/Scanned3DPeoplePack/RP_Character/rp_carla_rigged_001_ue4/rp_carla_rigged_001_ue4.rp_carla_rigged_001_ue4" :Option%201 "/Game/CityPark/Blueprints/Scanned3DPeoplePack/RP_Character/rp_claudia_rigged_002_ue4/rp_claudia_rigged_002_ue4.rp_claudia_rigged_002_ue4" :Option%202 "/Game/CityPark/Blueprints/Scanned3DPeoplePack/RP_Character/rp_eric_rigged_001_ue4/rp_eric_rigged_001_ue4.rp_eric_rigged_001_ue4" :Option%203 "/Game/CityPark/Blueprints/Scanned3DPeoplePack/RP_Character/rp_manuel_rigged_001_ue4/rp_manuel_rigged_001_ue4.rp_manuel_rigged_001_ue4" :Option%204 "/Game/CityPark/Blueprints/Scanned3DPeoplePack/RP_Character/rp_nathan_rigged_003_ue4/rp_nathan_rigged_003_ue4.rp_nathan_rigged_003_ue4" :Option%205 "/Game/CityPark/Blueprints/Scanned3DPeoplePack/RP_Character/rp_sophia_rigged_003_ue4/rp_sophia_rigged_003_ue4.rp_sophia_rigged_003_ue4") true)
  (Variables|Default|SetCurrent%20Speed (Variables|Default|GetWalking%20Speed)))

(event EventTick
  (params (DeltaSeconds :type Float%20%28single-precision%29))
  (CallFunction|CheckVeh))

(fn ConstructionScript)

(fn Stop
  (Variables|/Script/Engine.CharacterMovementComponent|SetMaxWalkSpeed (Variables|Character|GetCharacterMovement) 0.0))

(fn Walk
  (bind _walking_speed (Variables|Default|GetWalking%20Speed))
  (Variables|/Script/Engine.CharacterMovementComponent|SetMaxWalkSpeed (Variables|Character|GetCharacterMovement) _walking_speed)
  (Variables|Default|SetCurrent%20Speed _walking_speed))

(fn Run
  (bind _run_speed (Variables|Default|GetRun%20Speed))
  (Variables|/Script/Engine.CharacterMovementComponent|SetMaxWalkSpeed (Variables|Character|GetCharacterMovement) _run_speed)
  (Variables|Default|SetCurrent%20Speed _run_speed))

(fn Resume
  (Variables|/Script/Engine.CharacterMovementComponent|SetMaxWalkSpeed (Variables|Character|GetCharacterMovement) (Variables|Default|GetCurrent%20Speed)))