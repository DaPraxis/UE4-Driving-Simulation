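; CarStop is a traffic stop Blueprint that halts one AI_Car at a time with a trigger box.
; On begin overlap, it stores the first car, flags it TrafficStand and calls Stop.
; When any AI_Car ends overlap while triggered, it clears the stored car's flag, then after a short retriggerable delay frees the trigger and calls ResetDriving on that car.
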(event OnComponentEndOverlap(Box)
  (params (OverlappedComponent :type Primitive%20Component%20Object%20Reference) (OtherActor :type Actor%20Object%20Reference) (OtherComp :type Primitive%20Component%20Object%20Reference) (OtherBodyIndex :type Integer))
  (bind _triggered_car (Variables|Default|Gettriggered%20car))
  (if (and (Utilities|ClassIsChildOf (Utilities|GetClass OtherActor) "/Game/CityPark/Blueprints/BP/AI_Car.AI_Car_C") (Variables|Default|Getis%20triggered))
    (Variables|/Game/CityPark/Blueprints/BP/AI_Car.AI_Car_C|Settraffic_stand _triggered_car false)
    (Utilities|FlowControl|RetriggerableDelay 1.5)
    (Variables|Default|Setis%20triggered false)
    (Default|ResetDriving _triggered_car)))

(event OnComponentBeginOverlap(Box)
  (params (OverlappedComponent :type Primitive%20Component%20Object%20Reference) (OtherActor :type Actor%20Object%20Reference) (OtherComp :type Primitive%20Component%20Object%20Reference) (OtherBodyIndex :type Integer) (bFromSweep :type Boolean) (SweepResult :type Hit%20Result%20Structure%20%28by%20ref%29))
  (if (not (Variables|Default|Getis%20triggered))
    (bind _asai_car (Utilities|Casting|CastToAI_Car OtherActor))
    (Variables|/Game/CityPark/Blueprints/BP/AI_Car.AI_Car_C|Settraffic_stand _asai_car true)
    (Variables|Default|Setis%20triggered true)
    (Variables|Default|Settriggered%20car _asai_car)
    (Default|Stop _asai_car)))

(fn ConstructionScript)