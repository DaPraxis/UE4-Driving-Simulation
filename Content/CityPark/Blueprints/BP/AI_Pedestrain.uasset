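; AI controller that wanders a pedestrian between nearby points in the CityPark level.
; A multi-sphere object trace ahead of the pawn skips the current point, widening every 0.2 seconds until it hits.
; It stores a random hit actor as the current point and moves to a random reachable location around a separately randomized hit.
; Arrival triggers the next search immediately, while a failed move retries after a short delay.
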(event Custom|Go_to
  (params (Target :type Vector))
  (AI|AIMoveTo 0 Target 0 5e+01 false
    (:OnSuccess
      _)
    (:OnFail
      (Utilities|FlowControl|Delay 2.0)))
  (CallFunction|NextPoint))

(event EventBeginPlay
  (Utilities|FlowControl|Delay 1.0)
  (CallFunction|NextPoint))

(event EventTick
  (params (DeltaSeconds :type Float%20%28single-precision%29)))

(fn ConstructionScript)

(event Custom|Next_Point
  (bind _returnvalue (Pawn|GetControlledPawn))
  (bind _returnvalue_2 (Transformation|GetActorForwardVector _returnvalue))
  (bind _returnvalue_3 (Transformation|GetActorLocation _returnvalue))
  (bind _returnvalue_4 (* _returnvalue_2 700))
  (bind _returnvalue_5 (+ _returnvalue_3 _returnvalue_4))
  (Variables|Default|SetRadius (Variables|Default|GetDefaultRadius))
  (bind (_outhits _returnvalue_6) (Collision|MultiSphereTraceForObjects _returnvalue_5 (+ _returnvalue_5 "1.000000, 0, 0") (Variables|Default|GetRadius) (Utilities|Array|MakeArray "ObjectTypeQuery7") false (Utilities|Array|MakeArray (Variables|Default|Getcurrent_point)) "None" :!label _label))
  (if _returnvalue_6
    (Variables|Default|Setcurrent_point (.HitActor (Collision|BreakHitResult (Utilities|Array|Get(acopy) _outhits (Math|Random|RandomInteger (Utilities|Array|Length _outhits))))))
    (CallFunction|Goto (.RandomLocation (AI|Navigation|GetRandomReachablePointinRadius (.ImpactPoint (Collision|BreakHitResult (Utilities|Array|Get(acopy) _outhits (Math|Random|RandomInteger (Utilities|Array|Length _outhits))))) (Variables|Default|Getrandom_radius) 0 0)))
    (else
      (Variables|Default|SetRadius (+ (Variables|Default|GetRadius) (Variables|Default|GetExpand_radius)))
      (Utilities|FlowControl|Delay 0.2)
      (goto _label))))