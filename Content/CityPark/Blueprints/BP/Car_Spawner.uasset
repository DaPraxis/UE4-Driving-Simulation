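; Car spawner actor that places an AI car at its own transform when play begins.
; The Spawn function, guarded by a Spawned flag so it runs only once, creates an AI_Car pawn through SpawnAIFromClass.
; It then copies its Throttle value onto the new car and calls that car's own Spawn function.
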(event EventBeginPlay
  (CallFunction|Spawn))

(event Collision|EventActorBeginOverlap
  (params (OtherActor :type Actor%20Object%20Reference)))

(event EventTick
  (params (DeltaSeconds :type Float%20%28single-precision%29)))

(fn ConstructionScript)

(fn Spawn
  (bind _self self)
  (bind _returnvalue (Transformation|GetActorTransform _self))
  (if (not (Variables|Default|GetSpawned))
    (bind _returnvalue_2 (AI|SpawnAIFromClass "/Game/BP/AI_Car.AI_Car_C" 0 (.location _returnvalue) (.rotation _returnvalue) false 0))
    (Variables|Default|SetSpawned true)
    (bind _asai_car (Utilities|Casting|CastToAI_Car _returnvalue_2))
    (Variables|/Game/BP/AI_Car.AI_Car_C|SetThrottle _asai_car (Variables|Default|GetThrottle))
    (Default|Spawn _asai_car)))