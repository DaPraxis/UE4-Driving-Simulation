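; Actor that spawns a random number of pedestrian NPCs shortly after play begins.
; SpawnNPC loops with short delays, placing pedestrians at random reachable points around the spawner and giving each a default controller.
; It queries the GameState for available NPCs first, but that branch sets the NPC to None.
; Distance-based recycling into the GameState pool exists but never runs, and Tick spawning is disabled.
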(event Custom|Spawn%20NPC
  (Utilities|FlowControl|DoOnce false :!label _label
    (:Completed
      (if (> (Variables|Default|GetActual%20NPC%20amount) (Variables|Default|Getspawned%20npc%20count)) :!label _label_2
        (bind _npc (Class|BPINPCManagement|GetAvaliableNPCs(Message) (Game|GetGameState)))
        (Utilities|IsValid _npc
          (:Is%20Valid
            (Variables|Default|Settemp_npc 0))
          (:Is%20Not%20Valid
            (bind _returnvalue (Game|SpawnActorfromClass "/Game/CityPark/Blueprints/BP/Pedestrian.Pedestrian_C" (Math|Transform|MakeTransform (.RandomLocation (AI|Navigation|GetRandomReachablePointinRadius (Transformation|GetActorLocation) 5e+02 0 0)) (Math|Rotator|MakeRotator 0.0 0.0 (Math|Random|RandomFloatinRange 0.0 3.6e+02)) "1,1,1") "AdjustIfPossibleButDontSpawnIfColliding" 0 0))
            (Utilities|IsValid _returnvalue
              (:Is%20Valid
                (Variables|Default|Settemp_npc _returnvalue)))))
        (Utilities|Array|Add (Variables|Default|Getspawned%20npcs) (Variables|Default|Gettemp_npc))
        (Math|Integer|IncrementInt (Variables|Default|Getspawned%20npc%20count)
          (:%20%20
            (Utilities|FlowControl|Delay 0.2)
            (Pawn|SpawnDefaultController (Variables|Default|Gettemp_npc))
            (goto _label_2)))
        (else
          (goto _label Reset))))))

(event EventBeginPlay
  (bind _max_npc_count (Variables|Default|GetMax_NPC_Count))
  (Utilities|FlowControl|Delay (Math|Random|RandomFloatinRange 0.5 2.0))
  (if (== _max_npc_count 0)
    (Variables|Default|SetMin_NPC_Count 0))
  (Variables|Default|SetActual%20NPC%20amount (Math|Random|RandomIntegerinRange (Variables|Default|GetMin_NPC_Count) _max_npc_count))
  (Actor|Tick|SetActorTickEnabled true)
  (CallFunction|SpawnNPC))

(event Collision|EventActorBeginOverlap
  (params (OtherActor :type Actor%20Object%20Reference)))

(event EventTick
  (params (DeltaSeconds :type Float%20%28single-precision%29))
  (if false
    (CallFunction|SpawnNPC)))

(fn ConstructionScript)

(fn CheckNPCLocations
  (bind _spawned_npcs (Variables|Default|Getspawned%20npcs))
  (for _array_element _spawned_npcs
    (if (> (Utilities|GetDistancetoPlayer _array_element) (Variables|Default|Getnpc_range))
      (Class|BPINPCManagement|AddAvaliableNPCs(Message) (Game|GetGameState) _array_element)
      (Utilities|Array|RemoveItem _spawned_npcs _array_element)
      (Math|Integer|DecrementInt (Variables|Default|Getspawned%20npc%20count)))))