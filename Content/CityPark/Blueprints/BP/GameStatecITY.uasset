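; City Park game state that keeps a shared list of available NPCs.
; An event registers NPCs, adding each only once.
; The getter removes the first entry, then returns whatever is at index zero after removal, so it yields the following NPC rather than the removed one.
; An empty list returns no NPC.
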(event EventBeginPlay)

(event EventTick
  (params (DeltaSeconds :type Float%20%28single-precision%29)))

(event EventAddAvaliableNPCs
  (params (npc :type Pawn%20Object%20Reference))
  (Utilities|Array|AddUnique (Variables|Default|Getavailable_NPCs) npc))

(fn ConstructionScript)

(fn GetAvaliableNPCs
  (bind _available_npcs (Variables|Default|Getavailable_NPCs))
  (if (> (Utilities|Array|Length _available_npcs) 0)
    (Utilities|Array|RemoveIndex _available_npcs)
    (return (Utilities|Array|Get(acopy) _available_npcs))
    (else
      (return 0))))