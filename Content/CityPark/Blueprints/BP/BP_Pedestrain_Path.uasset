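; Pedestrian path actor that spawns a row of NPC_Point actors along its Path spline when play begins.
; A loop steps along the spline by Spacing until it reaches the end, storing each point in NpcPoints.
; Before respawning it clears that array and sets each old point's lifespan to zero, which does not destroy it.
; The construction script's placement call is disconnected.
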(event Custom|Place_NPC_Point
  (Variables|Default|SetDistance 0.0)
  (for _array_element (Variables|Default|Getnpc_points)
    (Actor|SetLifeSpan _array_element 0.0))
  (Utilities|Array|Clear (Variables|Default|Getnpc_points))
  (bind _returnvalue (Game|SpawnActorfromClass "/Game/CityPark/Blueprints/BP/NPC_Point.NPC_Point_C" (Math|Transform|MakeTransform (Spline|GetLocationatDistanceAlongSpline (Variables|Default|Getpath) (Variables|Default|GetDistance) "World") "0, 0, 0" "1,1,1") "Undefined" 0 0 :!label _label))
  (Utilities|Array|Add (Variables|Default|Getnpc_points) _returnvalue)
  (bind _output_get (Variables|Default|SetDistance (+ (Variables|Default|GetDistance) (Variables|Default|GetSpacing))))
  (if (< _output_get (Spline|GetSplineLength (Variables|Default|Getpath)))
    (goto _label)))

(event EventBeginPlay
  (CallFunction|PlaceNPCPoint))

(fn ConstructionScript)