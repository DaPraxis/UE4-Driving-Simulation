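; Traffic light controller for one side of a road, driving a group of vehicle lights, pedestrian lights and stop actors together.
; BeginPlay picks a random starting state, then loops Green, Yellow, Red using configurable delays.
; Each state switches the two-way and pedestrian lights and toggles collision on the car and pedestrian stop actors to block or release movement.
; Pedestrians get green only during car red, and yellow blocks both.
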(event EventBeginPlay
  (Variables|Default|SetCurrentTrafficState (Utilities|Enum|ByteToEnumTrafficLightEnum (Math|Conversions|ToByte(Integer) (Math|Random|RandomIntegerinRange 0 2))))
  (switch Utilities|FlowControl|Switch|SwitchonTrafficLightEnum (Variables|Default|GetCurrentTrafficState) :!label _label
    (:NewEnumerator0
      (Utilities|FlowControl|Sequence
        (:then_0
          (for _array_element (Variables|Default|GetTrafficLight)
            (bind _astwo_way_traffic_light (Utilities|Casting|CastToTwoWayTrafficLight _array_element))
            (Default|SwitchtoRed _astwo_way_traffic_light)))
        (:then_1
          (for _array_element_2 (Variables|Default|GetPedeLight)
            (bind _aspedestrian_traffic_light (Utilities|Casting|CastToPedestrianTrafficLight _array_element_2))
            (Default|SwitchtoGreen _aspedestrian_traffic_light)))
        (:then_2
          (for _array_element_3 (Variables|Default|GetCarStops)
            (Collision|SetActorEnableCollision _array_element_3 true)))
        (:then_3
          (for _array_element_4 (Variables|Default|GetPedStops)
            (Collision|SetActorEnableCollision _array_element_4 false)))
        (:then_4
          (Utilities|FlowControl|Delay (Variables|Default|GetRedTime))
          (Variables|Default|SetCurrentTrafficState "NewEnumerator2")
          (goto _label))))
    (:NewEnumerator1
      (Utilities|FlowControl|Sequence
        (:then_0
          (for _array_element_5 (Variables|Default|GetTrafficLight)
            (bind _astwo_way_traffic_light_2 (Utilities|Casting|CastToTwoWayTrafficLight _array_element_5))
            (Default|SwitchtoYellow _astwo_way_traffic_light_2)))
        (:then_1
          (for _array_element_6 (Variables|Default|GetCarStops)
            (Collision|SetActorEnableCollision _array_element_6 true)))
        (:then_2
          (for _array_element_7 (Variables|Default|GetPedStops)
            (Collision|SetActorEnableCollision _array_element_7 true)))
        (:then_3
          (for _array_element_8 (Variables|Default|GetPedeLight)
            (bind _aspedestrian_traffic_light_2 (Utilities|Casting|CastToPedestrianTrafficLight _array_element_8))
            (Default|SwitchtoRed _aspedestrian_traffic_light_2)))
        (:then_4
          (Utilities|FlowControl|Delay (Variables|Default|GetYellowTime))
          (Variables|Default|SetCurrentTrafficState "NewEnumerator0")
          (goto _label))))
    (:NewEnumerator2
      (Utilities|FlowControl|Sequence
        (:then_0
          (for _array_element_9 (Variables|Default|GetTrafficLight)
            (bind _astwo_way_traffic_light_3 (Utilities|Casting|CastToTwoWayTrafficLight _array_element_9))
            (Default|SwitchtoGreen _astwo_way_traffic_light_3)))
        (:then_1
          (for _array_element_10 (Variables|Default|GetPedeLight)
            (bind _aspedestrian_traffic_light_3 (Utilities|Casting|CastToPedestrianTrafficLight _array_element_10))
            (Default|SwitchtoRed _aspedestrian_traffic_light_3)))
        (:then_2
          (for _array_element_11 (Variables|Default|GetCarStops)
            (Collision|SetActorEnableCollision _array_element_11 false)))
        (:then_3
          (for _array_element_12 (Variables|Default|GetPedStops)
            (Collision|SetActorEnableCollision _array_element_12 true)))
        (:then_4
          (Utilities|FlowControl|Delay (Variables|Default|GetGreenTime))
          (Variables|Default|SetCurrentTrafficState "NewEnumerator1")
          (goto _label))))))

(fn ConstructionScript)